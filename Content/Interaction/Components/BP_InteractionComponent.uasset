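; Actor component that lets its owner interact with nearby objects implementing BPI_Interactable.
; On BeginPlay it finds the owner's sphere tagged "InteractionSphere" and binds its overlap events to maintain a list of interactables in range.
; Interact sends the interface Interact message to the first entry in that list, with no distance sorting or empty-list check.
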(event `self.ReceiveBeginPlay`
  (bind _output_get (set `self.InteractionCollision` (`|GetArrayItem` (`Actor.GetComponentsByTag` (`self.GetOwner`) "/Script/Engine.SphereComponent" "InteractionSphere"))))
  (add `PrimitiveComponent.OnComponentBeginOverlap` _output_get (delegate `AddInteractableToRange`))
  (add `PrimitiveComponent.OnComponentEndOverlap` (`self.InteractionCollision`) (delegate `RemoveInteractableFromRange`)))

(event `RemoveInteractableFromRange`
  (params (OverlappedComponent :type "PrimitiveComponent Object Reference") (OtherActor :type "Actor Object Reference") (OtherComp :type "PrimitiveComponent Object Reference") (OtherBodyIndex :type Integer))
  (`KismetArrayLibrary.Array_RemoveItem` (`self.InteractablesInRange`) OtherActor))

(event `AddInteractableToRange`
  (params (OverlappedComponent :type "PrimitiveComponent Object Reference") (OtherActor :type "Actor Object Reference") (OtherComp :type "PrimitiveComponent Object Reference") (OtherBodyIndex :type Integer) (bFromSweep :type Boolean) (SweepResult :type "HitResult Structure (by ref)"))
  (if (`KismetSystemLibrary.DoesImplementInterface` OtherActor "/Game/Interaction/Interfaces/BPI_Interactable.BPI_Interactable_C")
    (`KismetArrayLibrary.Array_AddUnique` (`self.InteractablesInRange`) OtherActor)))

(event `Interact`
  (message `/Game/Interaction/Interfaces/BPI_Interactable.Interact` (`|GetArrayItem` (`self.InteractablesInRange`))))